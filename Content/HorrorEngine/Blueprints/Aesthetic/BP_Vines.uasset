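; BP_Vines is a decorative vines actor for environment dressing, configured entirely in the Construction Script.
; The Type variable selects the plain master, thorns, or thorns-without-rose vine material for the Plane mesh.
; A dynamic instance of that material then receives VineColor, which is also pushed to three Niagara components so the effects match the vines.
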(fn `UserConstructionScript`
  (bind _plane (`self.Plane`))
  (bind _plane_2 (`self.Plane`))
  (bind _vinecolor (`self.VineColor`))
  (`|ExecutionSequence`
    (:`then_0`
      (switch `int` (`self.Type`)
        (:`0`
          (`PrimitiveComponent.SetMaterial` _plane 0 "/Game/Bee_Work/Materials/M_Vines_Master.M_Vines_Master"))
        (:`1`
          (`PrimitiveComponent.SetMaterial` _plane 0 "/Game/Bee_Work/Materials/M_Vines_Thorns.M_Vines_Thorns"))
        (:`2`
          (`PrimitiveComponent.SetMaterial` _plane 0 "/Game/Bee_Work/Materials/M_Vines_ThornsNoRose.M_Vines_ThornsNoRose"))))
    (:`then_1`
      (bind _returnvalue (`PrimitiveComponent.CreateDynamicMaterialInstance` _plane_2 0 (`PrimitiveComponent.GetMaterial` _plane_2 0) "None"))
      (`MaterialInstanceDynamic.SetVectorParameterValue` _returnvalue "Color" _vinecolor)
      (`NiagaraComponent.SetVariableLinearColor` (`self.Niagara1`) "Color" _vinecolor)
      (`NiagaraComponent.SetVariableLinearColor` (`self.Niagara2`) "Color" _vinecolor)
      (`NiagaraComponent.SetVariableLinearColor` (`self.Niagara`) "Color" _vinecolor))))